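; Player controller for the runner game that owns the HUD, pause menu and defeat screen.
; On BeginPlay it adds the HUD and binds to a death event, which pauses the game and GameMode timer, shows the defeat widget and saves the GameMode's time if it beats the stored best.
; The Pause input uses a FlipFlop to toggle pause, cursor and input mode, creating a new pause menu widget on each pause.
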(event Custom|DeathEvent
  (bind _asbp_runner_gm (CallFunction|GetGM))
  (bind _asbp_runner_gm_2 (CallFunction|GetGM))
  (bind _runner_pc (CallFunction|GetPC))
  (bind _gametime (Variables|/Script/Runner2.Runner2GameModeBase|GetGameTime _asbp_runner_gm))
  (bind _gametime_2 (Variables|/Script/Runner2.Runner2GameModeBase|GetGameTime _asbp_runner_gm_2))
  (Game|SetGamePaused true)
  (bind _returnvalue (UserInterface|CreateWidget "/Game/HUD/Menus/WBP_Defeat.WBP_Defeat_C"))
  (UserInterface|Viewport|AddtoViewport _returnvalue 0)
  (Variables|/Script/Engine.PlayerController|SetbShowMouseCursor _runner_pc true)
  (Input|SetInputModeUIOnly _runner_pc 0 "DoNotLock")
  (Utilities|Time|PauseTimerbyHandle (Variables|/Script/Runner2.Runner2GameModeBase|GettimerHandle (CallFunction|GetGM)))
  (bind _returnvalue_2 (SaveGame|DoesSaveGameExist "Game"))
  (if _returnvalue_2
    (bind _returnvalue_3 (SaveGame|LoadGamefromSlot "Game"))
    (bind _asbp_save_game (Utilities|Casting|CastToBP_SaveGame _returnvalue_3))
    (if (> _gametime_2 (Variables|/Game/Blueprints/GameSave/BP_SaveGame.BP_SaveGame_C|GetBestTimeInSeconds _asbp_save_game))
      (Variables|/Game/Blueprints/GameSave/BP_SaveGame.BP_SaveGame_C|SetBestTimeInSeconds _asbp_save_game _gametime_2)
      (SaveGame|SaveGametoSlot _asbp_save_game "Game"))
    (else
      (bind _returnvalue_4 (SaveGame|CreateSaveGameObject "/Game/Blueprints/GameSave/BP_SaveGame.BP_SaveGame_C"))
      (if (> _gametime (Variables|/Game/Blueprints/GameSave/BP_SaveGame.BP_SaveGame_C|GetBestTimeInSeconds _returnvalue_4))
        (Variables|/Game/Blueprints/GameSave/BP_SaveGame.BP_SaveGame_C|SetBestTimeInSeconds _returnvalue_4 _gametime)
        (SaveGame|SaveGametoSlot _returnvalue_4 "Game")))))

(event EventBeginPlay
  (EventDispatchers|BindEventtoDeath (delegate Custom|DeathEvent))
  (bind _returnvalue (UserInterface|CreateWidget "/Game/HUD/WBP_HUD.WBP_HUD_C"))
  (bind _output_get (Variables|Default|SetHUD_Ref _returnvalue))
  (UserInterface|Viewport|AddtoViewport _output_get 0))

(event EventTick
  (params (DeltaSeconds :type Float%20%28single-precision%29)))

(event Input|ActionEvents|InputActionPause
  (params (Key :type Key%20Structure :default "None"))
  (bind _self self)
  (:Pressed
    (Utilities|FlowControl|FlipFlop
      (:A
        (Game|SetGamePaused true)
        (Variables|Default|SetbShowMouseCursor true)
        (bind _returnvalue (UserInterface|CreateWidget "/Game/HUD/Menus/WBP_PauseMenu.WBP_PauseMenu_C"))
        (UserInterface|Viewport|AddtoViewport _returnvalue 0)
        (Input|SetInputModeUIOnly _self 0 "DoNotLock"))
      (:B
        (Game|SetGamePaused false)
        (Variables|Default|SetbShowMouseCursor false)
        (Input|SetInputModeGameOnly _self)))))

(fn ConstructionScript)