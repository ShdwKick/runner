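; BP_Destroyer is a volume that destroys BP_Obstacle actors once they stop overlapping its Cube component.
; It writes the Cube's world location and scale to the PC_Data Material Parameter Collection as "Position 1" and "Bound", exposing the volume to materials.
; The write runs in both the Construction Script and BeginPlay, so the values are set in the editor and at game start, with no per-frame update.
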(event OnComponentEndOverlap(Cube)
  (params (OverlappedComponent :type Primitive%20Component%20Object%20Reference) (OtherActor :type Actor%20Object%20Reference) (OtherComp :type Primitive%20Component%20Object%20Reference) (OtherBodyIndex :type Integer))
  (bind _asbp_obstacle (Utilities|Casting|CastToBP_Obstacle OtherActor))
  (Actor|DestroyActor _asbp_obstacle))

(event EventBeginPlay
  (bind _cube (Variables|Default|GetCube))
  (Rendering|Material|SetVectorParameterValue "/Game/Assets/MasterMaterials/Dissolve/PC_Data.PC_Data" "Position 1" (Math|Conversions|ToLinearColor(Vector) (Transformation|GetWorldLocation _cube)) :!class /Script/Engine.KismetMaterialLibrary)
  (Rendering|Material|SetVectorParameterValue "/Game/Assets/MasterMaterials/Dissolve/PC_Data.PC_Data" "Bound" (Math|Conversions|ToLinearColor(Vector) (Transformation|GetWorldScale _cube)) :!class /Script/Engine.KismetMaterialLibrary))

(event Collision|EventActorBeginOverlap
  (params (OtherActor :type Actor%20Object%20Reference)))

(event EventTick
  (params (DeltaSeconds :type Float%20%28single-precision%29)))

(fn ConstructionScript
  (bind _cube (Variables|Default|GetCube))
  (Rendering|Material|SetVectorParameterValue "/Game/Assets/MasterMaterials/Dissolve/PC_Data.PC_Data" "Position 1" (Math|Conversions|ToLinearColor(Vector) (Transformation|GetWorldLocation _cube)) :!class /Script/Engine.KismetMaterialLibrary)
  (Rendering|Material|SetVectorParameterValue "/Game/Assets/MasterMaterials/Dissolve/PC_Data.PC_Data" "Bound" (Math|Conversions|ToLinearColor(Vector) (Transformation|GetWorldScale _cube)) :!class /Script/Engine.KismetMaterialLibrary))